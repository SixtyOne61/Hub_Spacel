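; BP_FlyingGameMode is the game mode that spawns and possesses BP_ShipPawn ships for players in the flying game.
; On the server, a new player gets a ship at the spawn location for the team stored in their SpacelPlayerState.
; OnRestartPlayer waits a fixed delay, then spawns a fresh ship at the supplied transform, has the controller possess it and calls Restarted on it.
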(event EventBeginPlay)

(event EventTick
  (params (DeltaSeconds :type Float%20%28single-precision%29)))

(event EventHandleStartingNewPlayer
  (params (NewPlayer :type Player%20Controller%20Object%20Reference))
  (Networking|SwitchHasAuthority
    (:Authority
      (bind _asspacel_player_state (Utilities|Casting|CastToSpacelPlayerState (Variables|/Script/Engine.Controller|GetPlayerState NewPlayer)))
      (bind _returnvalue (Class|FlyingGameMode|GetSpawnLocation (Utilities|String|StringToName (Variables|/Script/Hub_Spacel.SpacelPlayerState|GetTeam _asspacel_player_state))))
      (bind _returnvalue_2 (Game|SpawnActorfromClass "/Game/Blueprint/Pawn/BP_ShipPawn.BP_ShipPawn_C" _returnvalue "AlwaysSpawn" NewPlayer 0))
      (Pawn|Possess NewPlayer _returnvalue_2))))

(event EventOnRestartPlayer
  (params (_controller :type Controller%20Object%20Reference) (_transform :type Transform%20%28by%20ref%29))
  (Networking|SwitchHasAuthority
    (:Authority
      (Utilities|FlowControl|Delay 5.0)
      (bind _returnvalue (Game|SpawnActorfromClass "/Game/Blueprint/Pawn/BP_ShipPawn.BP_ShipPawn_C" _transform "AlwaysSpawn" _controller 0))
      (Pawn|Possess _controller _returnvalue)
      (Class|ShipPawn|Restarted _returnvalue))))

(fn ConstructionScript)