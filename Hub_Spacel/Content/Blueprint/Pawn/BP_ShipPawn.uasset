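; Player ship pawn that adds sound and UI feedback to ship events and builds the default ship in its construction script.
; Fx events play FMOD components for firing, matter pickup and effect voice lines, with plain sound assets for matter loss and death.
; Hit and damage events spawn viewport indicator widgets, and F presses the interaction widget pointer; its release is unwired.
; InitFireComponent hands five Katyusha dummy locations to the fire component.
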(event EventBeginPlay)

(event Collision|EventActorBeginOverlap
  (params (OtherActor :type Actor%20Object%20Reference)))

(event EventFxRemoveEffect
  (params (_effect :type EEffect%20Enum :default "None"))
  ;[1 1 1] Sound
  (switch Utilities|FlowControl|Switch|SwitchonEEffect _effect
    (:TargetLock
      (Class|FMODAudioComponent|Play (Variables|Default|GetFMODVoiceTargetLost)))))

(event EventDamageIndicator
  (params (_location :type Vector%20%28by%20ref%29 :default "0, 0, 0"))
  (bind (_x _y) (Math|Vector|BreakVector _location))
  (bind _self self)
  (bind _returnvalue (UserInterface|CreateWidget "/Game/Blueprint/UI/Widgets/Player/Hit_Indicator/WBP_DamageIndicator.WBP_DamageIndicator_C" (Game|GetPlayerController 0) _self (Math|Vector|MakeVector _x _y (.Z (Math|Vector|BreakVector (Transformation|GetActorLocation _self))))))
  (UserInterface|Viewport|AddtoViewport _returnvalue 0))

(event EventHitIndicator
  (bind _returnvalue (UserInterface|CreateWidget "/Game/Blueprint/UI/Widgets/Player/Hit_Indicator/WBP_HitIndicator.WBP_HitIndicator_C" (Game|GetPlayerController 0)))
  (UserInterface|Viewport|AddtoViewport _returnvalue 0))

(event EventInitFireComponent
  ;[1 1 1] Init Fire Component
  (Variables|/Script/Hub_Spacel.FireComponent|SetDummyKatyushaLocations (Variables|Default|GetFireComponent) (Utilities|Array|MakeArray (Variables|Default|GetDummyKatyusha01) (Variables|Default|GetDummyKatyusha02) (Variables|Default|GetDummyKatyusha03) (Variables|Default|GetDummyKatyusha04) (Variables|Default|GetDummyKatyusha05))))

(event EventTick
  (params (DeltaSeconds :type Float%20%28single-precision%29)))

(event EventOnStartGame
  ;[1 1 1] Sound
  (Class|FMODAudioComponent|Play (Variables|Default|GetFMODVoiceWelcome)))

(event EventFxFireBullet
  ;[1 1 1] Sound
  (Class|FMODAudioComponent|Play (Variables|Default|GetFMODBasicShot)))

(event EventFxFireMissile
  ;[1 1 1] Sound
  (Class|FMODAudioComponent|Play (Variables|Default|GetFMODSecondaryShot)))

(event EventFxAddMatiere
  (params (_val :type Integer))
  ;[1 1 1] Sound
  (if (> _val 0)
    (Class|FMODAudioComponent|Play (Variables|Default|GetFMODMatterLoot))
    (else
      (Audio|PlaySound2D "/Game/Sound/FX/Beep/RemoveMatter_01.RemoveMatter_01" 0.1 1.0 0.0 0 0))))

(event EventFxKilled
  ;[1 1 1] Sound
  (Audio|PlaySoundatLocation "/Game/Sound/FX/Ship/Destroy_01.Destroy_01" (Transformation|GetActorLocation) "0, 0, 0" 0.3 1.0 0.0 0 0 0))

(event EventFxAddEffect
  (params (_effect :type EEffect%20Enum :default "None"))
  ;[1 1 1] Sound
  (switch Utilities|FlowControl|Switch|SwitchonEEffect _effect
    (:Fog
      (Class|FMODAudioComponent|Play (Variables|Default|GetFMODVoiceFog)))))

(event Input|KeyboardEvents|F
  (params (Key :type Key%20Structure :default "None"))
  (:Pressed
    (Class|WidgetInteractionComponent|PressPointerKey (Variables|Default|GetInteractionWidget) Key)))

(fn ConstructionScript
  (Class|ShipPawn|BuildDefaultShip))